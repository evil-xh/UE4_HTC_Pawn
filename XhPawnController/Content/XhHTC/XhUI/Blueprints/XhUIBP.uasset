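; XhUIBP is an HTC VR UI manager actor that tracks buttons in its XhUI widget components.
; After a short delay on BeginPlay, it maps each component's buttons and boolean log states by name, saving an initial copy for resets.
; Functions query hover (bypassed by the HTC pawn's debug flag) and get or set log states.
; A timeline animates widget scale; hover binding and style setup are disconnected.
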(event `self.ReceiveDestroyed`
  (`/XhPawnController/XhHTC/XhMacro/XhMacroF.XhPrintMsg` "UI已被销毁！！！"))

(event `self.ReceiveBeginPlay`
  (`self.XhButtonsInital`))

(event `XhButtonHovered`
  ;[1 1 1] 注释     按钮初始化
  (`/XhPawnController/XhHTC/XhMacro/XhMacroF.XhPrintMsg` "有一个按钮被指向了！！！"))

(event `XhButtonsInital`
  ;[1 1 1] 注释     按钮初始化
  (`KismetSystemLibrary.Delay` 0.5)
  (for _array_element (`SceneComponent.GetChildrenComponents` (`self.DefaultSceneRoot`) true)
    (bind _output_get (set `self.SceneComponent` _array_element))
    (bind _aswidget_component (cast `WidgetComponent` _output_get)
      (:`then`
        (bind _asxh_ui (cast `/XhPawnController/XhHTC/XhUI/Widget/XhUI` (`WidgetComponent.GetUserWidgetObject` _aswidget_component)))
        (set `self.XhUI` _asxh_ui)
        (bind _output_get_2 (set `self.XhLoopButtons` (`/XhPawnController/XhHTC/XhUI/Widget/XhUI.XhButtons` _asxh_ui)))
        (for _array_element_2 _output_get_2
          (set `self.XhLoopButton` _array_element_2)
          (`BlueprintMapLibrary.Map_Add` (`self.XhButtonLog`) (`KismetSystemLibrary.GetObjectName` (`self.XhLoopButton`))))
        (`BlueprintMapLibrary.Map_Add` (`self.XhUIButtons`) (`KismetSystemLibrary.GetObjectName` (`self.SceneComponent`)) (make `/XhPawnController/XhHTC/XhStruct/XhUIButtons` (`self.XhLoopButtons`)))
        (`BlueprintMapLibrary.Map_Add` (`self.XhUIButtonsLog`) (`KismetSystemLibrary.GetObjectName` (`self.SceneComponent`)) (make `/XhPawnController/XhHTC/XhStruct/XhUIButtonLog` (`self.XhButtonLog`)))
        (`BlueprintMapLibrary.Map_Clear` (`self.XhButtonLog`)))
      (:`CastFailed`
        (`/XhPawnController/XhHTC/XhMacro/XhMacroF.XhPrintWarn` "此蓝图需要与XhUI一同使用！！！"))))
  (set `self.XhUIButtonsInitalLog` (`self.XhUIButtonsLog`))
  (`/XhPawnController/XhHTC/XhMacro/XhMacroF.XhPrintMsg` "按钮初始化完成！！！"))

(event `XhWidgetTransform`
  (params (WidgetComponent :type "WidgetComponent Object Reference") (Time :type "Float (double-precision)" :default 1.0) (OldScale :type "Vector Structure") (NewScale :type "Vector Structure") (Reverse :type Boolean))
  ;[1 1 1] 注释     UI变换
  (`TimelineComponent.SetPlayRate` (`self.XhWidgetTransformTimeLine`) (/ 1.0 Time))
  (if Reverse
    (bind (_direction _transform) (`Timeline|XhWidgetTransformTimeLine` :!via `ReverseFromEnd` :!label _label)
      (:`Update`
        (`SceneComponent.SetRelativeScale3D` WidgetComponent (`KismetMathLibrary.VLerp` OldScale NewScale _transform)))
      (:`Finished`
        (`/XhPawnController/XhHTC/XhMacro/XhMacroF.XhPrintMsg` "变换已完成！！！")))
    (else
      (goto _label :!via `PlayFromStart`))))

(fn `UserConstructionScript`)

(fn `XhClearButtonsLog`
  (`BlueprintMapLibrary.Map_Clear` (`self.XhUIButtonsLog`))
  (set `self.XhUIButtonsLog` (`self.XhUIButtonsInitalLog`)))

(fn `XhGetButtonsLog`
  (params (UIName :type String) (ButtonName :type String))
  (returns (ReturnValue :type Boolean))
  (locals (LoopButtonLog :type "/XhPawnController/XhHTC/XhStruct/XhUIButtonLog Structure"))
  (bind (_value _returnvalue) (`BlueprintMapLibrary.Map_Find` (`self.XhUIButtonsLog`) UIName))
  (bind (_value_2 _returnvalue_2) (`BlueprintMapLibrary.Map_Find` (`.ButtonLog_19_CB3DC36345C157CE46A8B3A7FD19D640` (break `/XhPawnController/XhHTC/XhStruct/XhUIButtonLog` _value)) ButtonName))
  (if _returnvalue
    (if _returnvalue_2
      (return _value_2)
      (else
        (`/XhPawnController/XhHTC/XhMacro/XhMacroF.XhPrintWarn` "没有此按钮！！！")))
    (else
      (`/XhPawnController/XhHTC/XhMacro/XhMacroF.XhPrintWarn` "没有此UI！！！"))))

(fn `XhIsHoverButton`
  (params (UIName :type String) (ButtonName :type String))
  (returns (ReturnValue :type Boolean))
  (locals (IsHover :type Boolean) (XhButtons :type "/XhPawnController/XhHTC/XhStruct/XhUIButtons Structure"))
  (bind (_value _returnvalue) (`BlueprintMapLibrary.Map_Find` (`self.XhUIButtons`) UIName))
  (if _returnvalue
    (set `local.XhButtons` _value)
    (bind _outactors (`GameplayStatics.GetAllActorsOfClass` "/XhPawnController/XhHTC/XhPawn/Blueprints/XhHTCPawn.XhHTCPawn_C"))
    (if (`/XhPawnController/XhHTC/XhPawn/Blueprints/XhHTCPawn.IsUIDebug` (`|GetArrayItem` _outactors))
      (`/XhPawnController/XhHTC/XhMacro/XhMacroF.XhPrintMsg` "已打开跳过UI设置！！！")
      (return true)
      (else
        (for _array_element (`.Buttons_3_13C1CE004762D105B30E908D29860797` (break `/XhPawnController/XhHTC/XhStruct/XhUIButtons` (`local.XhButtons`)))
          (if (and (`KismetStringLibrary.EqualEqual_StrStr` (`KismetSystemLibrary.GetObjectName` _array_element) ButtonName) (`Widget.IsHovered` _array_element))
            (set `local.IsHover` true)
            (break)))
        (if (`local.IsHover`)
          (return (`local.IsHover`)))))
    (else
      (`/XhPawnController/XhHTC/XhMacro/XhMacroF.XhPrintWarn` "没有此UI！！！"))))

(fn `XhSetButtonExtendStyle`
  (params (Button :type "Button Object Reference") (Scale :type "Float (double-precision)"))
  (`Widget.SetRenderScale` Button (* (`.Scale` (break `WidgetTransform` (`Widget.RenderTransform` Button))) Scale)))

(fn `XhSetButtonsLog`
  (params (UIName :type String) (ButtonName :type String) (SetValue :type Boolean))
  (locals (LoopButtonLog :type "/XhPawnController/XhHTC/XhStruct/XhUIButtonLog Structure") (IsFind :type Boolean) (Index :type Integer) (ButtonLogIndex :type Integer))
  (bind (_value _returnvalue) (`BlueprintMapLibrary.Map_Find` (`self.XhUIButtonsLog`) UIName))
  (if _returnvalue
    (if (`.ReturnValue` (`BlueprintMapLibrary.Map_Find` (`.ButtonLog_19_CB3DC36345C157CE46A8B3A7FD19D640` (break `/XhPawnController/XhHTC/XhStruct/XhUIButtonLog` _value)) ButtonName))
      (`BlueprintMapLibrary.Map_Add` (`.ButtonLog_19_CB3DC36345C157CE46A8B3A7FD19D640` (break `/XhPawnController/XhHTC/XhStruct/XhUIButtonLog` (`BlueprintMapLibrary.Map_Find` (`self.XhUIButtonsLog`) UIName))) ButtonName SetValue)
      (`BlueprintMapLibrary.Map_Add` (`self.XhUIButtonsLog`) UIName (`BlueprintMapLibrary.Map_Find` (`self.XhUIButtonsLog`) UIName))
      (else
        (`/XhPawnController/XhHTC/XhMacro/XhMacroF.XhPrintWarn` "没有此按钮！！！")))
    (else
      (`/XhPawnController/XhHTC/XhMacro/XhMacroF.XhPrintWarn` "没有此UI！！！"))))