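; XhDirectionRouteBP is a direction route actor that lays sign meshes along a spline, with a destination mesh and a view sign.
; The construction script spawns evenly spaced, spline-aligned sign meshes when the count exceeds one.
; It then shows the destination and child ViewSignBP, passing the latter its float distance and mesh.
; Box overlap events record an overlap flag and their event data in variables.
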(event `self.Box.OnComponentBeginOverlap`
  (params (OverlappedComponent :type "PrimitiveComponent Object Reference") (OtherActor :type "Actor Object Reference") (OtherComp :type "PrimitiveComponent Object Reference") (OtherBodyIndex :type Integer) (bFromSweep :type Boolean) (SweepResult :type "HitResult Structure (by ref)"))
  (set `self.IsOverlap` true)
  (set `self.BeginOverlappedComponent` OverlappedComponent)
  (set `self.BeginOtherActor` OtherActor)
  (set `self.BeginOtherComponent` OtherComp)
  (set `self.BeginOtherBodyIndex` OtherBodyIndex)
  (set `self.BeginFormSweep` bFromSweep)
  (set `self.BeginSweepResult` SweepResult))

(event `self.Box.OnComponentEndOverlap`
  (params (OverlappedComponent :type "PrimitiveComponent Object Reference") (OtherActor :type "Actor Object Reference") (OtherComp :type "PrimitiveComponent Object Reference") (OtherBodyIndex :type Integer))
  (set `self.IsOverlap` false)
  (set `self.EndOverlappedComponent` OverlappedComponent)
  (set `self.EndOtherActor` OtherActor)
  (set `self.EndOtherComponent` OtherComp)
  (set `self.EndOtherBodyIndex` OtherBodyIndex))

(fn `UserConstructionScript`
  (bind _number_of_mesh (`self.Number Of Mesh`))
  (bind _spline (`self.Spline`))
  (bind _returnvalue (* (`self.ForIndex`) (/ (`SplineComponent.GetSplineLength` (`self.Spline`)) (`KismetMathLibrary.Conv_IntToDouble` (- (`self.Number Of Mesh`) 1)))))
  (`StaticMeshComponent.SetStaticMesh` (`self.StaticMesh`) (`self.Destination`))
  (if (> _number_of_mesh 1)
    (for _index (range _number_of_mesh)
      (set `self.ForIndex` _index)
      (bind _returnvalue_2 (`AddComponent|NODE_AddStaticMeshComponent-3` :`RelativeTransform` (`KismetMathLibrary.MakeTransform` (`SplineComponent.GetLocationAtDistanceAlongSpline` _spline _returnvalue "Local") (struct) (* (`self.SignScale`) (`self.SignSize`)))))
      (`StaticMeshComponent.SetStaticMesh` _returnvalue_2 (`self.MoveSign`))
      (`SceneComponent.K2_SetWorldRotation` _returnvalue_2 (`SplineComponent.GetRotationAtDistanceAlongSpline` _spline _returnvalue "World") false false))
    (`SceneComponent.SetVisibility` (`self.ChildActor`) true false)
    (`SceneComponent.SetVisibility` (`self.StaticMesh`) true false)
    (bind _asview_sign_bp (cast `/XhPawnController/XhHTC/XhDirectionRoute/BluePrints/ViewSignBP` (`ChildActorComponent.ChildActor` (`self.ChildActor`))))
    (set `/XhPawnController/XhHTC/XhDirectionRoute/BluePrints/ViewSignBP.FloatDistance` (`self.FloatDistance`) _asview_sign_bp)
    (`StaticMeshComponent.SetStaticMesh` (`/XhPawnController/XhHTC/XhDirectionRoute/BluePrints/ViewSignBP.StaticMesh` _asview_sign_bp) (`self.ViewSign`))))