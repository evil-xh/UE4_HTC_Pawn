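; ViewSignBP is a sign actor whose static mesh bobs up and down continuously.
; BeginPlay caches the mesh's relative location as the center of the motion.
; Tick passes through a DoOnce into two chained one-second MoveComponentTo calls, raising then lowering the mesh by FloatDistance around that center at unchanged rotation.
; The DoOnce resets after the second move, so the cycle repeats without a Timeline.
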(event `self.ReceiveBeginPlay`
  (set `self.Oldlocation` (`SceneComponent.RelativeLocation` (`self.StaticMesh`))))

(event `self.ReceiveTick`
  (params (DeltaSeconds :type "Float (single-precision)"))
  (bind (_oldlocation_x _oldlocation_y _oldlocation_z) (`KismetMathLibrary.BreakVector` (`self.Oldlocation`)))
  (bind (_oldlocation_x_2 _oldlocation_y_2 _oldlocation_z_2) (`KismetMathLibrary.BreakVector` (`self.Oldlocation`)))
  (`/Engine/EditorBlueprintResources/StandardMacros.DoOnce` false :!label _label
    (:`Completed`
      (`KismetSystemLibrary.MoveComponentTo` (`self.StaticMesh`) (`KismetMathLibrary.MakeVector` _oldlocation_x _oldlocation_y (+ _oldlocation_z (`self.FloatDistance`))) (`SceneComponent.RelativeRotation` (`self.StaticMesh`)) false false 1.0)
      (`KismetSystemLibrary.MoveComponentTo` (`self.StaticMesh`) (`KismetMathLibrary.MakeVector` _oldlocation_x_2 _oldlocation_y_2 (- _oldlocation_z_2 (`self.FloatDistance`))) (`SceneComponent.RelativeRotation` (`self.StaticMesh`)) false false 1.0)
      (goto _label :!via `Reset`))))

(fn `UserConstructionScript`)