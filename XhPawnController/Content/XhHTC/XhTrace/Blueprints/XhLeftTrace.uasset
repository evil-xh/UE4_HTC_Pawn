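; XhLeftTrace is the left-hand laser pointer for the HTC VR pawn, XhHTCPawn.
; Each tick it snaps to the left motion controller and sets its WidgetInteraction active from the pawn's ComplexTraceL flag.
; Its visibility line trace stretches the beam mesh to the hit or maximum distance and shows a marker mesh on blocking hits.
; Hit static mesh actors and components are written back to the pawn.
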(event `self.ReceiveBeginPlay`
  (bind _outactors (`GameplayStatics.GetAllActorsOfClass` "/XhPawnController/XhHTC/XhPawn/Blueprints/XhHTCPawn.XhHTCPawn_C"))
  (set `self.Player` (`|GetArrayItem` _outactors))
  (`SceneComponent.SetWorldScale3D` (`self.ComplexTrace`) (`KismetMathLibrary.MakeVector` (/ (`self.Size`) 157.0) (/ (`self.Size`) 273.0) (/ (`self.Size`) 288.0))))

(event `self.ReceiveTick`
  (params (DeltaSeconds :type "Float (single-precision)"))
  (`|ExecutionSequence`
    (:`then_0`
      (`self.XhMakeTrace` (`self.ComplexTrace`) self (`self.HitStaticMesh`) (`self.Size`)))
    (:`then_1`
      (`ActorComponent.SetActive` (`self.WidgetInteraction`) (`/XhPawnController/XhHTC/XhPawn/Blueprints/XhHTCPawn.ComplexTraceL` (`self.Player`)) false))
    (:`then_2`
      (`SceneComponent.K2_SetWorldTransform` (`self.DefaultSceneRoot`) (`SceneComponent.K2_GetComponentToWorld` (`/XhPawnController/XhHTC/XhPawn/Blueprints/XhHTCPawn.LeftMotionController` (`self.Player`))) false false))))

(fn `UserConstructionScript`
  (bind (_returnvalue_x _returnvalue_y _returnvalue_z) (`KismetMathLibrary.BreakVector` (`SceneComponent.K2_GetComponentScale` (`self.ComplexTrace`))))
  (`SceneComponent.SetWorldScale3D` (`self.ComplexTrace`) (`KismetMathLibrary.MakeVector` _returnvalue_x (* (`self.Size`) _returnvalue_y) (* (`self.Size`) _returnvalue_z)))
  (`ParticleSystemComponent.SetTemplate` (`self.ParticleSystem`) (`self.NewParticleSystem`))
  (`PrimitiveComponent.SetMaterial` (`self.ComplexTrace`) 0 (`self.NewMaterial`)))

(fn `XhMakeTrace`
  (params (ComplexTrace :type "StaticMeshComponent Object Reference") (SelfActor :type "Actor Object Reference") (HitStaticMesh :type "StaticMeshComponent Object Reference") (Size :type "Float (double-precision)"))
  (bind (_returnvalue_x _returnvalue_y _returnvalue_z) (`KismetMathLibrary.BreakVector` (`SceneComponent.K2_GetComponentScale` ComplexTrace)))
  (bind _leftstyle (`/XhPawnController/XhHTC/XhPawn/Blueprints/XhHTCPawn.LeftStyle` (`self.Player`)))
  (bind _leftstyle_2 (`/XhPawnController/XhHTC/XhPawn/Blueprints/XhHTCPawn.LeftStyle` (`self.Player`)))
  (bind _returnvalue (`SceneComponent.K2_GetComponentLocation` _leftstyle_2))
  (bind _outhit (`KismetSystemLibrary.LineTraceSingle` _returnvalue (+ _returnvalue (* (`KismetMathLibrary.Conv_RotatorToVector` (`SceneComponent.K2_GetComponentRotation` _leftstyle_2)) (`BlueprintMapLibrary.Map_Find` (`/XhPawnController/XhHTC/XhPawn/Blueprints/XhHTCPawn.ComplexTraceDistance` (`self.Player`)) "NewEnumerator0"))) "TraceTypeQuery1" false (`|MakeArray` SelfActor)))
  (bind (_bblockinghit _binitialoverlap _time _distance _location _impactpoint _normal _impactnormal _physmat _hitactor _hitcomponent) (`GameplayStatics.BreakHitResult` _outhit))
  (if _bblockinghit
    (`SceneComponent.SetWorldScale3D` ComplexTrace (`KismetMathLibrary.MakeVector` (/ _distance 156.0) _returnvalue_y _returnvalue_z))
    (`SceneComponent.K2_SetWorldLocation` HitStaticMesh (+ (`SceneComponent.K2_GetComponentLocation` _leftstyle) (* (`KismetMathLibrary.Conv_RotatorToVector` (`SceneComponent.K2_GetComponentRotation` _leftstyle)) (- _distance 2.0))) false false)
    (`SceneComponent.SetHiddenInGame` HitStaticMesh false false)
    (bind _asstatic_mesh_actor (cast `StaticMeshActor` _hitactor)
      (:`then`
        (set `/XhPawnController/XhHTC/XhPawn/Blueprints/XhHTCPawn.XhLeftTraceHitActor` _asstatic_mesh_actor (`self.Player`)))
      (:`CastFailed`
        _))
    (bind _asstatic_mesh_component (cast `StaticMeshComponent` _hitcomponent)
      (:`then`
        (set `/XhPawnController/XhHTC/XhPawn/Blueprints/XhHTCPawn.XhLeftTraceHitComponent` _asstatic_mesh_component (`self.Player`)))
      (:`CastFailed`
        _))
    (return)
    (else
      (`SceneComponent.SetWorldScale3D` ComplexTrace (`KismetMathLibrary.MakeVector` (/ (`BlueprintMapLibrary.Map_Find` (`/XhPawnController/XhHTC/XhPawn/Blueprints/XhHTCPawn.ComplexTraceDistance` (`self.Player`)) "NewEnumerator0") 156.0) (/ Size 273.0) (/ Size 288.0)))
      (`SceneComponent.SetHiddenInGame` HitStaticMesh true false)
      (return))))